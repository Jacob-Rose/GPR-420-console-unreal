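; BP_WeatherActor drives sky, lighting, rain and weather UI from a requested weather forecast.
; Construction makes dynamic material instances for the volumetric cloud and directional light function; BeginPlay sends the weather request.
; Every Tick, it searches the first period's short forecast for "Cloudy" and "Rain" to set cloud noise, a light parameter (name unset) and rain spawn intensity.
; It also passes that forecast to BP_Player's WeatherUI.
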(event `self.ReceiveBeginPlay`
  (`self.SendWeatherRequest`))

(event `self.ReceiveTick`
  (params (DeltaSeconds :type "Float (single-precision)"))
  (bind (_updated _cwa _periods) (break `WeatherForecast` (`self.m_UpdatedWeatherForecast`)))
  (bind (_name _starttime _isdaytime _temperature _temperatureunit _shortforecast) (break `WeatherPeriod` (`|GetArrayItem` _periods)))
  (bind _returnvalue (`KismetStringLibrary.Contains` _shortforecast "Cloudy"))
  (if (> (`KismetArrayLibrary.Array_Length` _periods) 0)
    (bind _asmaterial_instance_dynamic (cast `MaterialInstanceDynamic` (`VolumetricCloudComponent.Material` (`self.VolumetricCloud`)))
      (:`then`
        (`MaterialInstanceDynamic.SetScalarParameterValue` _asmaterial_instance_dynamic "BaseNoiseExp" (`KismetMathLibrary.SelectFloat` 20.0 150.0 _returnvalue))
        (bind _asmaterial_instance_dynamic_2 (cast `MaterialInstanceDynamic` (`LightComponent.LightFunctionMaterial` (`self.DirectionalLight`))))
        (`MaterialInstanceDynamic.SetScalarParameterValue` _asmaterial_instance_dynamic_2 "None" (`KismetMathLibrary.SelectFloat` -4.0 0.95 _returnvalue))
        (`FXSystemComponent.SetFloatParameter` (`self.Rain`) "SpawnIntensity" (`KismetMathLibrary.SelectFloat` 1.0 0.0 (`KismetStringLibrary.Contains` _shortforecast "Rain"))) ; Param = 1 if raining
        (bind _asbp_player (cast `/Game/Blueprints/BP_Player` (`Controller.K2_GetPawn` (`GameplayStatics.GetPlayerController` 0))))
        (`/Game/Blueprints/BP_UIWidget.CheckWeather` (`/Game/Blueprints/BP_Player.Weather UI` _asbp_player) _shortforecast))
      (:`CastFailed`
        (`KismetSystemLibrary.PrintString` "Cast Failed")))))

(fn `UserConstructionScript`
  (bind _volumetriccloud (`self.VolumetricCloud`))
  (bind _returnvalue (`KismetMaterialLibrary.CreateDynamicMaterialInstance` (`VolumetricCloudComponent.Material` _volumetriccloud)))
  (`VolumetricCloudComponent.SetMaterial` _volumetriccloud _returnvalue)
  (bind _returnvalue_2 (`KismetMaterialLibrary.CreateDynamicMaterialInstance` (`LightComponent.LightFunctionMaterial` (`self.DirectionalLight`))))
  (`LightComponent.SetLightFunctionMaterial` (`self.DirectionalLight`) _returnvalue_2))