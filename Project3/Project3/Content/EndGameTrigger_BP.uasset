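; End-of-level trigger for the ball-rolling game that finishes the level when the BallRollingPawn overlaps it.
; It flags LevelOver on BallGM, records the timer with username and date, then calls ChangeLevel with LevelID.
; SaveLevelTime creates a per-level save slot, or appends the run when a stored time is lower.
; An existing slot is only re-saved when the list exceeds five entries and gets trimmed.
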(event `self.ReceiveActorBeginOverlap`
  (params (OtherActor :type "Actor Object Reference"))
  (cast `BallRollingPawn` OtherActor)
  (`self.LevelFinished`))

(fn `LevelFinished`
  (locals (PlayerStat :type "/Game/PlayerTime Structure"))
  (bind _asball_gm (cast `/Game/BallGM` (`GameplayStatics.GetGameMode`)))
  (set `/Game/BallGM.LevelOver` true _asball_gm)
  (bind _asball_game_instance (cast `/Game/BallGameInstance` (`GameplayStatics.GetGameInstance`)))
  (`self.SaveLevelTime` (make `/Game/PlayerTime` (`/Game/BallGameInstance.PlayerUsername` _asball_game_instance) (`KismetMathLibrary.Now`) (`KismetMathLibrary.FromSeconds` (`/Game/BallGM.Timer` _asball_gm))) (`self.LevelID`))
  (`MiscFunctionLibrary.ChangeLevel` self (`self.LevelID`)))

(fn `SaveLevelTime`
  (params (PlayerInfo :type "/Game/PlayerTime Structure") (Level :type Integer))
  (returns (Successful :type Boolean))
  (bind _returnvalue (`KismetStringLibrary.Concat_StrStr` "Level" (`KismetStringLibrary.Conv_IntToString` Level) "Saves"))
  (bind _returnvalue_2 (`GameplayStatics.DoesSaveGameExist` _returnvalue))
  (if _returnvalue_2
    (bind _returnvalue_3 (`GameplayStatics.LoadGameFromSlot` _returnvalue))
    (bind _aslevel_save_state (cast `/Game/LevelSaveState` _returnvalue_3))
    (bind _levelsaves (`/Game/LevelSaveState.LevelSaves` _aslevel_save_state))
    (for _array_element _levelsaves
      (`/Engine/EditorBlueprintResources/StandardMacros.CompareFloat` (`KismetMathLibrary.GetTotalSeconds` (`.Time_8_748D3B9A4E9B26FDD0B70BAD20D95FAF` (break `/Game/PlayerTime` _array_element))) (`KismetMathLibrary.GetTotalSeconds` (`.Time_8_748D3B9A4E9B26FDD0B70BAD20D95FAF` (break `/Game/PlayerTime` PlayerInfo)))
        (:`<`
          (`KismetArrayLibrary.Array_Add` _levelsaves PlayerInfo)
          (if (> (`KismetArrayLibrary.Array_Length` _levelsaves) 5)
            (`KismetArrayLibrary.Array_Resize` _levelsaves 5)
            (bind _returnvalue_4 (`GameplayStatics.SaveGameToSlot` _aslevel_save_state _returnvalue))
            (return (or _returnvalue_4 (stale _returnvalue_6)))))))
    (else
      (bind _returnvalue_5 (`GameplayStatics.CreateSaveGameObject` "/Game/LevelSaveState.LevelSaveState_C"))
      (`KismetArrayLibrary.Array_Add` (`/Game/LevelSaveState.LevelSaves` _returnvalue_5) PlayerInfo)
      (bind _returnvalue_6 (`GameplayStatics.SaveGameToSlot` _returnvalue_5 _returnvalue))
      (return (or _returnvalue_4 _returnvalue_6)))))

(fn `UserConstructionScript`)